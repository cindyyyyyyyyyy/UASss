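; BP_Shooter is a shooter actor that automatically fires projectiles at a repeating interval.
; Tick runs into a Delay set by a variable, which ignores re-triggers while pending and so acts as a fire-rate timer before calling the shoot event.
; The event spawns PanahAtauLaser at the Sphere component's world location, rotated along the actor's forward vector.
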(event `self.ReceiveTick`
  (params (DeltaSeconds :type "Float (single-precision)"))
  (`KismetSystemLibrary.Delay` (`self.Delay`))
  (`self.shoot_laser`))

(event `shoot_laser`
  (`|SpawnActorFromClass` (`self.Panah Atau Laser`) (`KismetMathLibrary.MakeTransform` (`SceneComponent.K2_GetComponentLocation` (`self.Sphere`)) (`KismetMathLibrary.MakeRotFromX` (`self.GetActorForwardVector`))) "Undefined" "OverrideRootScale" null null))

(fn `UserConstructionScript`)
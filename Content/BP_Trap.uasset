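; BP_Trap is a trigger actor that switches shooters on when the first-person character overlaps it.
; Begin overlap enables actor tick on every BP_Shooter tagged ShooterTag, so those shooters need no direct references.
; End overlap disables their tick again, but only if the BERHENTIENGGA boolean (Indonesian for "stop or not") is true.
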(event `self.ReceiveActorBeginOverlap`
  (params (OtherActor :type "Actor Object Reference"))
  (if (`KismetMathLibrary.ClassIsChildOf` (`GameplayStatics.GetObjectClass` OtherActor) "/Game/FirstPersonBP/Blueprints/FirstPersonCharacter.FirstPersonCharacter_C")
    (bind _outactors (`GameplayStatics.GetAllActorsOfClassWithTag` "/Game/BP_Shooter.BP_Shooter_C" (`self.ShooterTag`)))
    (`self.SetActorTickEnabled` _outactors true)))

(event `self.ReceiveActorEndOverlap`
  (params (OtherActor :type "Actor Object Reference"))
  (if (`self.BERHENTI ENGGA`)
    (if (`KismetMathLibrary.ClassIsChildOf` (`GameplayStatics.GetObjectClass` OtherActor) "/Game/FirstPersonBP/Blueprints/FirstPersonCharacter.FirstPersonCharacter_C")
      (bind _outactors (`GameplayStatics.GetAllActorsOfClassWithTag` "/Game/BP_Shooter.BP_Shooter_C" (`self.ShooterTag`)))
      (`self.SetActorTickEnabled` _outactors false))))

(fn `UserConstructionScript`)
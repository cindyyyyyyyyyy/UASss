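; BP_Laser is a laser actor that affects the first-person character on contact.
; On overlap with a FirstPersonCharacter, it passes itself to that character's CheckLaserOverlapHealth, then destroys itself.
; The health logic lives in the character, and other overlapping actors are ignored.
; A three-second self-destruct chain is present but unconnected, so it never runs.
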(event `self.ReceiveBeginPlay`)

(event `self.ReceiveActorBeginOverlap`
  (params (OtherActor :type "Actor Object Reference"))
  (if (`KismetMathLibrary.ClassIsChildOf` (`GameplayStatics.GetObjectClass` OtherActor) "/Game/FirstPersonBP/Blueprints/FirstPersonCharacter.FirstPersonCharacter_C")
    (bind _asfirst_person_character (cast `/Game/FirstPersonBP/Blueprints/FirstPersonCharacter` OtherActor))
    (`/Game/FirstPersonBP/Blueprints/FirstPersonCharacter.CheckLaserOverlapHealth` _asfirst_person_character self)
    (`self.K2_DestroyActor`)))

(fn `UserConstructionScript`)